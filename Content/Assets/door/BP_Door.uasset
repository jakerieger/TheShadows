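; BP_Door is an interactive door that the E key opens and closes while something overlaps its proximity collider.
; A FlipFlop alternates playing and reversing a timeline that drives DoorRoot's yaw, with a sound for each direction.
; Overlap begin creates an on-screen prompt widget and overlap end removes it.
; A second FlipFlop on timeline completion switches the prompt text between open and close and sets IsDoorOpen.
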(event `Key|E` :consume false
  (params (Key :type "Key Structure" :default "AnyKey"))
  (bind _returnvalue (`SceneComponent.K2_GetComponentLocation` (`self.DefaultSceneRoot`)))
  (bind _interacttext (`/Game/Assets/UI/InteractPromps.interactText` (`self.InteractivePrompt`)))
  (:`Pressed`
    (if (`self.CanOpenDoor?`)
      (`/Engine/EditorBlueprintResources/StandardMacros.FlipFlop`
        (:`A`
          (`GameplayStatics.PlaySoundAtLocation` "/Game/Assets/Sound/Door/CUE_DoorOpen.CUE_DoorOpen" _returnvalue)
          (bind (_direction _rotationamount) (`Timeline|OpenDoorTimeline` :!via `PlayFromStart` :!label _label)
            (:`Update`
              (`SceneComponent.K2_SetRelativeRotation` (`self.DoorRoot`) (`KismetMathLibrary.MakeRotator` 0.0 0.0 _rotationamount) false false))
            (:`Finished`
              (`/Engine/EditorBlueprintResources/StandardMacros.FlipFlop`
                (:`A`
                  (bind _output_get (set `self.DoorPromptText` "[E] CLOSE DOOR"))
                  (`TextBlock.SetText` _interacttext _output_get :!label _label_2)
                  (set `self.isDoorOpen` false))
                (:`B`
                  (bind _output_get_2 (set `self.DoorPromptText` "[E] OPEN DOOR"))
                  (`TextBlock.SetText` _interacttext _output_get_2 :!label _label_3)
                  (set `self.isDoorOpen` true))))))
        (:`B`
          (`GameplayStatics.PlaySoundAtLocation` "/Game/Assets/Sound/Door/CUE_DoorClose.CUE_DoorClose" _returnvalue)
          (goto _label :!via `ReverseFromEnd`))))))

(event `self.ProximityCollider.OnComponentBeginOverlap`
  (params (OverlappedComponent :type "PrimitiveComponent Object Reference") (OtherActor :type "Actor Object Reference") (OtherComp :type "PrimitiveComponent Object Reference") (OtherBodyIndex :type Integer) (bFromSweep :type Boolean) (SweepResult :type "HitResult Structure (by ref)"))
  (set `self.CanOpenDoor?` true)
  (bind _returnvalue (`|CreateWidget` "/Game/Assets/UI/InteractPromps.InteractPromps_C"))
  (bind _output_get (set `self.InteractivePrompt` _returnvalue))
  (`UserWidget.AddToViewport` _output_get 0)
  (if (`self.isDoorOpen`)
    (goto _label_2)
    (else
      (goto _label_3))))

(event `self.ProximityCollider.OnComponentEndOverlap`
  (params (OverlappedComponent :type "PrimitiveComponent Object Reference") (OtherActor :type "Actor Object Reference") (OtherComp :type "PrimitiveComponent Object Reference") (OtherBodyIndex :type Integer))
  (set `self.CanOpenDoor?` false)
  (`Widget.RemoveFromParent` (stale `self.ProximityCollider.OnComponentBeginOverlap` _returnvalue)))

(fn `UserConstructionScript`)